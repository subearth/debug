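; Self-opening door actor that sinks out of the way when something overlaps its DoorOpener trigger while CanDoorOpen is set.
; The overlap sets OpenDoor, then Tick slides Door along local -Z at DoorOpenSpeed until DistanceTraveled reaches OpenDistance.
; It then marks the door open and destroys the Top, Bottom and Door components, so it never closes again.
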(event OnComponentBeginOverlap(DoorOpener)
  (params (OverlappedComponent :type Primitive%20Component%20Object%20Reference) (OtherActor :type Actor%20Object%20Reference) (OtherComp :type Primitive%20Component%20Object%20Reference) (OtherBodyIndex :type Integer) (bFromSweep :type Boolean) (SweepResult :type Hit%20Result%20Structure%20%28by%20ref%29))
  ;[1 1 1] At the door
  (if (Variables|Default|GetCan%20Door%20Open)
    (Variables|Default|SetOpen%20Door true)))

(event EventBeginPlay)

(event Collision|EventActorBeginOverlap
  (params (OtherActor :type Actor%20Object%20Reference)))

(event EventTick
  (params (DeltaSeconds :type Float%20%28single-precision%29))
  (bind _door_open_speed (Variables|Default|GetDoor%20Open%20Speed))
  (bind _returnvalue (* DeltaSeconds _door_open_speed))
  ;[1 1 1] Open the door
  (if (and (not (Variables|Default|GetDoor%20Open)) (Variables|Default|GetOpen%20Door))
    (if (< (Variables|Default|GetDistance%20Traveled) (Variables|Default|GetOpen%20Distance))
      (Transformation|AddLocalOffset (Variables|Default|GetDoor) (Math|Vector|MakeVector 0.0 0.0 (* _returnvalue -1.0)) false true)
      (Variables|Default|SetDistance%20Traveled (+ _returnvalue (Variables|Default|GetDistance%20Traveled)))
      (else
        (Variables|Default|SetDoor%20Open true)
        (Components|DestroyComponent (Variables|Default|GetTop))
        (Components|DestroyComponent (Variables|Default|GetDoor))))))

(fn ConstructionScript)