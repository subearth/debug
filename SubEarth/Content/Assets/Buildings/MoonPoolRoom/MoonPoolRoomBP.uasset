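; Moon pool room building Blueprint with a pair of sliding doors that can be opened.
; On BeginPlay it registers itself with the MoonpoolPanel child actor of its ControlPanel component.
; The open event, guarded against repeat triggers while open or moving, plays a rate-scaled timeline that slides the two doors in opposite directions along relative X up to a maximum distance.
; No closing logic is present.
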(event Custom|EventOpenMoonpoolDoor
  (bind _doorclose (Variables|Default|GetDoorClose))
  (bind _doorfar (Variables|Default|GetDoorFar))
  (bind _relativelocation (Variables|/Script/Engine.SceneComponent|GetRelativeLocation _doorclose))
  (bind _relativelocation_2 (Variables|/Script/Engine.SceneComponent|GetRelativeLocation _doorfar))
  ;[1 1 1] If door is not opened or opening, play the opening animation
  (if (and (not (Variables|Default|GetbDoorOpened)) (not (Variables|Default|GetbDoorMoving)))
    (Components|Timeline|SetPlayRate (Variables|Default|GetDoorOpenTimeline) (Variables|Default|GetDoorOpenTimeFactor))
    (Variables|Default|SetbDoorMoving true)
    (bind _dooropenscale (Timeline|DoorOpenTimeline Play)
      (:Update
        (Transformation|SetRelativeLocation _doorclose (Math|Vector|MakeVector (* _dooropenscale (Variables|Default|GetDoorOpenMaxDistance)) (.y _relativelocation) (.z _relativelocation)) false false)
        (Transformation|SetRelativeLocation _doorfar (Math|Vector|MakeVector (* (* _dooropenscale (Variables|Default|GetDoorOpenMaxDistance)) -1.0) (.y _relativelocation_2) (.z _relativelocation_2)) false false))
      (:Finished
        (Variables|Default|SetbDoorOpened (not (Variables|Default|GetbDoorOpened)))
        (Variables|Default|SetbDoorMoving false)))))

(event EventBeginPlay
  ;[1 1 1] Register self to the control panel
  (bind _asmoonpool_panel (Utilities|Casting|CastToMoonpoolPanel (Variables|/Script/Engine.ChildActorComponent|GetChildActor (Variables|Default|GetControlPanel))))
  (Variables|/Game/Assets/Objects/ControlPanelA/MoonpoolPanel.MoonpoolPanel_C|SetMoonpoolRoomReference _asmoonpool_panel self))

(event Collision|EventActorBeginOverlap
  (params (OtherActor :type Actor%20Object%20Reference)))

(event EventTick
  (params (DeltaSeconds :type Float%20%28single-precision%29)))

(fn ConstructionScript)