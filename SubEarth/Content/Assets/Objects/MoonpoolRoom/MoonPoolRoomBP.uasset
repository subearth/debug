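; MoonPoolRoomBP is the moonpool room actor, with a pair of sliding doors opened by an event.
; On BeginPlay it registers itself with the MoonpoolPanel held in its ControlPanel child actor, giving the panel a reference to the room.
; EventOpenMoonpoolDoor plays a timeline that slides Door1 and Door2 apart along local Y, using DoorOpened and DoorMoving flags to block retriggering; no closing path exists.
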(event Custom|EventOpenMoonpoolDoor
  ;[1 1 1] If door is not opened or opening, play the opening animation
  (if (and (not (Variables|Default|GetbDoorOpened)) (not (Variables|Default|GetbDoorMoving)))
    (Variables|Default|SetbDoorMoving true)
    (bind _doorlocation (Timeline|DoorOpenTimeline PlayFromStart)
      (:Update
        (Transformation|SetRelativeLocation (Variables|Default|GetDoor%202) (Math|Vector|MakeVector 0.0 _doorlocation 0.0) false false)
        (Transformation|SetRelativeLocation (Variables|Default|GetDoor%201) (* (Math|Vector|MakeVector 0.0 _doorlocation 0.0) -1.0) false false))
      (:Finished
        (Variables|Default|SetbDoorOpened (not (Variables|Default|GetbDoorOpened)))
        (Variables|Default|SetbDoorMoving false)))))

(event EventBeginPlay
  ;[1 1 1] Register self to the control panel
  (bind _asmoonpool_panel (Utilities|Casting|CastToMoonpoolPanel (Variables|/Script/Engine.ChildActorComponent|GetChildActor (Variables|Default|GetControlPanel))))
  (Variables|/Game/Assets/Objects/ControlPanelA/MoonpoolPanel.MoonpoolPanel_C|SetMoonpoolRoomReference _asmoonpool_panel self))

(event Collision|EventActorBeginOverlap
  (params (OtherActor :type Actor%20Object%20Reference)))

(event EventTick
  (params (DeltaSeconds :type Float%20%28single-precision%29)))

(fn ConstructionScript)