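; Air pocket Blueprint that builds a configurable water surface, seen from above and below, using two mesh components.
; The construction script calls InitialWaterCreation, which gives WaterSurface and WaterSubSurface dynamic instances of OceanMaterial and scales both in X and Y.
; It then pushes shared wave, color, depth and opacity settings to both materials.
; Each takes its water height from its component's world Z, and the underside negates shore depth.
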(fn ConstructionScript
  (bind _below_water_material (Variables|Default|GetBelow%20Water%20Material))
  (bind _below_water_material_2 (Variables|Default|GetBelow%20Water%20Material))
  (bind _above_water_material (Variables|Default|GetAbove%20Water%20Material))
  (bind _above_water_material_2 (Variables|Default|GetAbove%20Water%20Material))
  (|InitialWaterCreation)
  (for _index (range 0 1)
    (switch int _index
      (:0
        (Rendering|Material|SetScalarParameterValue _above_water_material "Shore Depth" (Variables|Default|GetShore%20Depth) :!class /Script/Engine.MaterialInstanceDynamic)
        (Rendering|Material|SetScalarParameterValue _above_water_material "Wave Speed" (Variables|Default|GetWave%20Speed) :!class /Script/Engine.MaterialInstanceDynamic)
        (Rendering|Material|SetScalarParameterValue _above_water_material "BaseOpacity" (Variables|Default|GetBase%20Opacity) :!class /Script/Engine.MaterialInstanceDynamic)
        (Rendering|Material|SetScalarParameterValue _above_water_material "Water Height" (.Z (Math|Vector|BreakVector (Transformation|GetWorldLocation (Variables|Default|GetWaterSurface)))) :!class /Script/Engine.MaterialInstanceDynamic)
        (Rendering|Material|SetScalarParameterValue _above_water_material "Water Scale" (Variables|Default|GetOverall%20Water%20Scale) :!class /Script/Engine.MaterialInstanceDynamic)
        (Rendering|Material|SetScalarParameterValue _above_water_material "Variation Amount" (Variables|Default|GetVariation%20Amount) :!class /Script/Engine.MaterialInstanceDynamic)
        (Rendering|Material|SetVectorParameterValue _above_water_material "WaterColor A" (Variables|Default|GetPrimary%20Water%20Color) :!class /Script/Engine.MaterialInstanceDynamic)
        (Rendering|Material|SetVectorParameterValue _above_water_material "WaterColor B" (Variables|Default|GetSecondary%20Water%20Color) :!class /Script/Engine.MaterialInstanceDynamic)
        (Rendering|Material|SetScalarParameterValue _above_water_material_2 "Water Depth" (Variables|Default|GetDepth%20Scale) :!class /Script/Engine.MaterialInstanceDynamic)
        (Rendering|Material|SetVectorParameterValue _above_water_material_2 "DeepWater" (Variables|Default|GetDeep%20Water%20Color) :!class /Script/Engine.MaterialInstanceDynamic)
        (Rendering|Material|SetVectorParameterValue _above_water_material_2 "ShallowWater" (Variables|Default|GetShallow%20Water%20Color) :!class /Script/Engine.MaterialInstanceDynamic))
      (:1
        (Rendering|Material|SetScalarParameterValue _below_water_material_2 "Shore Depth" (* (Variables|Default|GetShore%20Depth) -1.0) :!class /Script/Engine.MaterialInstanceDynamic)
        (Rendering|Material|SetScalarParameterValue _below_water_material_2 "Wave Speed" (Variables|Default|GetWave%20Speed) :!class /Script/Engine.MaterialInstanceDynamic)
        (Rendering|Material|SetScalarParameterValue _below_water_material_2 "BaseOpacity" (Variables|Default|GetBase%20Opacity) :!class /Script/Engine.MaterialInstanceDynamic)
        (Rendering|Material|SetScalarParameterValue _below_water_material_2 "Water Height" (.Z (Math|Vector|BreakVector (Transformation|GetWorldLocation (Variables|Default|GetWaterSubSurface)))) :!class /Script/Engine.MaterialInstanceDynamic)
        (Rendering|Material|SetScalarParameterValue _below_water_material_2 "Water Scale" (Variables|Default|GetOverall%20Water%20Scale) :!class /Script/Engine.MaterialInstanceDynamic)
        (Rendering|Material|SetScalarParameterValue _below_water_material_2 "Variation Amount" (Variables|Default|GetVariation%20Amount) :!class /Script/Engine.MaterialInstanceDynamic)
        (Rendering|Material|SetVectorParameterValue _below_water_material_2 "WaterColor A" (Variables|Default|GetPrimary%20Water%20Color) :!class /Script/Engine.MaterialInstanceDynamic)
        (Rendering|Material|SetVectorParameterValue _below_water_material_2 "WaterColor B" (Variables|Default|GetSecondary%20Water%20Color) :!class /Script/Engine.MaterialInstanceDynamic)
        (Rendering|Material|SetScalarParameterValue _below_water_material "Water Depth" (Variables|Default|GetDepth%20Scale) :!class /Script/Engine.MaterialInstanceDynamic)
        (Rendering|Material|SetVectorParameterValue _below_water_material "DeepWater" (Variables|Default|GetDeep%20Water%20Color) :!class /Script/Engine.MaterialInstanceDynamic)
        (Rendering|Material|SetVectorParameterValue _below_water_material "ShallowWater" (Variables|Default|GetShallow%20Water%20Color) :!class /Script/Engine.MaterialInstanceDynamic)))))