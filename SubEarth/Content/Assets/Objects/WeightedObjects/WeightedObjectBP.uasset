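; Physics object for an elevator puzzle that adds its weight to the elevator it lands on.
; An overlap with the elevator's tagged collider, or with another weighted object already on it, stores the elevator reference, adds the weight and registers as last touched.
; Stacked objects pass the reference along, and weight is zeroed after giving so it counts once.
; Tick applies extra downward acceleration during vertical movement to make it sink faster.
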(event OnComponentBeginOverlap(OverlappingMesh)
  (params (OverlappedComponent :type Primitive%20Component%20Object%20Reference) (OtherActor :type Actor%20Object%20Reference) (OtherComp :type Primitive%20Component%20Object%20Reference) (OtherBodyIndex :type Integer) (bFromSweep :type Boolean) (SweepResult :type Hit%20Result%20Structure%20%28by%20ref%29))
  ;[1 1 1] Landed on the elevator
  (if (Components|ComponentHasTag OtherComp "Weighted Objects Collider")
    (bind _aselevator_puzzle_bp (Utilities|Casting|CastToElevatorPuzzleBP OtherActor))
    (Variables|Default|SetElevator%20Reference _aselevator_puzzle_bp)
    (Variables|Default|SetOn%20Elevator true)
    ;[1 1 1] Add our weight to the elevator
    (Default|AddWeight (stale _output_get) (Variables|Default|GetWeight%20To%20Give) :!label _label)
    (Variables|Default|SetWeight%20To%20Give 0.0)
    (Default|SetLastObjectTouched (Variables|Default|GetElevator%20Reference) self)
    (else
      ;[1 1 1] Landed on another weighted object
      (if (Components|ComponentHasTag OtherComp "Weighted Object")
        (bind _asweighted_object_bp (Utilities|Casting|CastToWeightedObjectBP OtherActor))
        ;[1 1 1] We landed on one that is on the elevator
        (if (Variables|WeightedObjectBP_C|GetOn%20Elevator _asweighted_object_bp)
          (Variables|Default|SetOn%20Elevator true)
          (bind _output_get (Variables|Default|SetElevator%20Reference (Variables|WeightedObjectBP_C|GetElevator%20Reference _asweighted_object_bp)))
          (goto _label))))))

(event EventBeginPlay)

(event Collision|EventActorBeginOverlap
  (params (OtherActor :type Actor%20Object%20Reference)))

(event EventTick
  (params (DeltaSeconds :type Float%20%28single-precision%29))
  ;[1 1 1] Sink faster
  (if (> (Math|Float|Absolute(Float) (.Z (Math|Vector|BreakVector (Transformation|GetComponentVelocity (Variables|Default|GetObject%20Mesh))))) 1.0)
    (Physics|AddForce (Variables|Default|GetObject%20Mesh) (Math|Vector|MakeVector 0.0 0.0 (* DeltaSeconds -1.5e+04)) "None" true)))

(fn ConstructionScript)