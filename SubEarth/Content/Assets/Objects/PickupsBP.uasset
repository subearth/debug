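; Pickup object that drifts by alternately sinking and floating, and lights up when found by sonar.
; While its mesh simulates physics, Tick applies a vertical force for the current mode plus random torque.
; Overlapping world-static geometry zeroes its velocity and flips the mode.
; Sonar-tagged overlaps swap all materials to a sonar material, then restore the originals cached at BeginPlay after a short delay.
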(event OnComponentBeginOverlap(StaticMesh)
  (params (OverlappedComponent :type Primitive%20Component%20Object%20Reference) (OtherActor :type Actor%20Object%20Reference) (OtherComp :type Primitive%20Component%20Object%20Reference) (OtherBodyIndex :type Integer) (bFromSweep :type Boolean) (SweepResult :type Hit%20Result%20Structure%20%28by%20ref%29))
  ;[1 1 1] Hit stuff in the world
  (for _index (range 0 1)
    (switch int _index
      (:0
        (if (Utilities|Enum|Equal(Enum) (Collision|GetCollisionObjectType OtherComp) "ECC_WorldStatic")
          (Class|PrimitiveComponent|SetAllPhysicsLinearVelocity (Variables|Default|GetStaticMesh) "0, 0, 0" false)
          (if (== (Variables|Pickups|GetMovement%20Mode%20Value) (Variables|Default|GetSinking%20Mode%20Value))
            (Variables|Pickups|SetMovement%20Mode%20Value (Variables|Default|GetFloating%20Mode%20Value))
            (else
              (Variables|Pickups|SetMovement%20Mode%20Value (Variables|Default|GetSinking%20Mode%20Value))))))
      (:1
        ;[1 1 1] Found by sonar
        (if (Components|ComponentHasTag OtherComp "Sonar")
          (for _index_2 (range 0 1)
            (switch int _index_2
              (:0
                ;[1 1 1] show object via sonar
                (for _index_3 (range 0 (Rendering|Material|GetNumMaterials (Variables|Default|GetStaticMesh)))
                  (Rendering|Material|SetMaterial (Variables|Default|GetStaticMesh) _index_3 "/Game/Assets/Materials/SonarPickupMaterial.SonarPickupMaterial")))
              (:1
                ;[1 1 1] Restore the objects original materials
                (Utilities|FlowControl|Delay 5.0)
                (for _index_4 (range 0 (Rendering|Material|GetNumMaterials (Variables|Default|GetStaticMesh)))
                  (Rendering|Material|SetMaterial (Variables|Default|GetStaticMesh) _index_4 (Utilities|Array|Get(acopy) (Variables|Default|GetSaved%20Materials) _index_4)))))))))))

(event EventBeginPlay
  ;[1 1 1] Initialize the location
  (Variables|Default|SetLast%20Position (Transformation|GetWorldLocation (Variables|Default|GetStaticMesh)))
  ;[1 1 1] Save the original materials for the pickup
  (for _index (range 0 (Rendering|Material|GetNumMaterials (Variables|Default|GetStaticMesh)))
    (bind _asmaterial (Utilities|Casting|CastToMaterial (Rendering|Material|GetMaterial (Variables|Default|GetStaticMesh) _index)))
    (Utilities|Array|Add (Variables|Default|GetSaved%20Materials) _asmaterial)))

(event Collision|EventActorBeginOverlap
  (params (OtherActor :type Actor%20Object%20Reference)))

(event EventTick
  (params (DeltaSeconds :type Float%20%28single-precision%29))
  ;[1 1 1] Floating and sinking simulation
  (Variables|Default|SetTick%20Time DeltaSeconds)
  (if (Class|SceneComponent|IsAnySimulatingPhysics (Variables|Default|GetStaticMesh))
    (if (== (Variables|Pickups|GetMovement%20Mode%20Value) (Variables|Default|GetSinking%20Mode%20Value))
      ;[1 1 1] Sink
      (Physics|AddForce (Variables|Default|GetStaticMesh) (Math|Vector|MakeVector 0.0 0.0 (* (Variables|Pickups|GetSink%20Speed) (Variables|Default|GetTick%20Time))) "None" true)
      (else
        ;[1 1 1] Float
        (Physics|AddForce (Variables|Default|GetStaticMesh) (Math|Vector|MakeVector 0.0 0.0 (* (Variables|Pickups|GetFloat%20Speed) (Variables|Default|GetTick%20Time))) "None" true)))
    ;[1 1 1] Rotate
    (Class|PrimitiveComponent|AddTorque (Variables|Default|GetStaticMesh) (* (Math|Random|RandomUnitVector) (* (Variables|Pickups|GetRotate%20Speed) (Variables|Default|GetTick%20Time))) "None" true)))

(fn ConstructionScript)

(fn PressButtonLeft
  (params (NewParam :type Boolean)))

(fn PressButtonRight
  (params (NewParam :type Boolean)))

(fn PressButtonDown)

(fn SetVisibility
  (params (Visibility :type Boolean))
  (bind _staticmesh (Variables|Default|GetStaticMesh))
  (Development|SetHiddeninGame _staticmesh (not Visibility) true)
  (Rendering|SetVisibility _staticmesh Visibility true))