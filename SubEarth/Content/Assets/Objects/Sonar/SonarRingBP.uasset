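; SonarRingBP is a sonar ring actor that grows and travels in a set direction, then destroys itself after TimeToDeath.
; Each Tick scales Sphere1 toward MaxScale on a cubic curve of elapsed lifetime, so growth starts slow and speeds up.
; The Scene offset grows with elapsed time and is not scaled by delta time, so movement accelerates and depends on frame rate.
; BeginPlay saves StartLocation, which this graph never reads.
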(event EventBeginPlay
  ;[1 1 1] Save where we spawned at
  (Variables|Default|SetStart%20Location (Transformation|GetWorldLocation (Variables|Default|GetSphere1))))

(event Collision|EventActorBeginOverlap
  (params (OtherActor :type Actor%20Object%20Reference)))

(event EventTick
  (params (DeltaSeconds :type Float%20%28single-precision%29))
  (bind _output_get (Variables|Default|SetTime%20Used (+ DeltaSeconds (Variables|Default|GetTime%20Used))))
  (if (>= _output_get (Variables|Default|GetTime%20to%20Death))
    (Actor|DestroyActor)
    (else
      (Transformation|SetWorldScale3D (Variables|Default|GetSphere1) (* (Variables|Default|GetMax%20Scale) (Math|Float|Power (/ (Variables|Default|GetTime%20Used) (Variables|Default|GetTime%20to%20Death)) 3.0)))
      (Transformation|AddWorldOffset (Variables|Default|GetScene) (* (Variables|Default|GetDirection%20To%20Move) (* (Variables|Default|GetMovement%20speed) _output_get)) false false))))

(fn ConstructionScript)