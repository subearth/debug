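; Toolbox actor whose lid swings open and shut in response to overlaps with two trigger components.
; Overlapping BoxOpener rolls the lid mesh toward its opened angle on Tick, and leaving it starts a stay-out timer.
; Once the timer expires, the lid auto-closes if between the closed and max-fall angles.
; From max-fall or beyond, it closes only after BoxCloser is overlapped.
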(event OnComponentBeginOverlap(BoxOpener)
  (params (OverlappedComponent :type Primitive%20Component%20Object%20Reference) (OtherActor :type Actor%20Object%20Reference) (OtherComp :type Primitive%20Component%20Object%20Reference) (OtherBodyIndex :type Integer) (bFromSweep :type Boolean) (SweepResult :type Hit%20Result%20Structure%20%28by%20ref%29))
  ;[1 1 1] Collide with the box opener and closer
  (Variables|Default|SetIs%20Opening true)
  (Variables|Default|SetIs%20Closing false)
  (Variables|Default|SetIs%20Out false))

(event OnComponentBeginOverlap(BoxCloser)
  (params (OverlappedComponent :type Primitive%20Component%20Object%20Reference) (OtherActor :type Actor%20Object%20Reference) (OtherComp :type Primitive%20Component%20Object%20Reference) (OtherBodyIndex :type Integer) (bFromSweep :type Boolean) (SweepResult :type Hit%20Result%20Structure%20%28by%20ref%29))
  ;[1 1 1] Collide with the box opener and closer
  (Variables|Default|SetIs%20Closing true)
  (Variables|Default|SetIs%20Opening false))

(event OnComponentEndOverlap(BoxOpener)
  (params (OverlappedComponent :type Primitive%20Component%20Object%20Reference) (OtherActor :type Actor%20Object%20Reference) (OtherComp :type Primitive%20Component%20Object%20Reference) (OtherBodyIndex :type Integer))
  ;[1 1 1] Collide with the box opener and closer
  (Variables|Default|SetIs%20Out true)
  (Variables|Default|SetCurrent%20Time 0.0))

(event EventBeginPlay)

(event Collision|EventActorBeginOverlap
  (params (OtherActor :type Actor%20Object%20Reference)))

(event EventTick
  (params (DeltaSeconds :type Float%20%28single-precision%29))
  ;[1 1 1] Are we outside the box
  (Variables|Default|SetDelta%20Time DeltaSeconds)
  (if (Variables|Default|GetIs%20Out)
    ;[1 1 1] Have we been out long enough
    (bind _output_get (Variables|Default|SetCurrent%20Time (+ (Variables|Default|GetCurrent%20Time) (Variables|Default|GetDelta%20Time))))
    (if (> _output_get (Variables|Default|GetStay%20Out%20Time))
      ;[1 1 1] Are we at an angle we should auto close at?
      (if (and (> (Variables|Default|GetCurrent%20Angle) (Variables|Default|GetClosed%20Angle)) (< (Variables|Default|GetCurrent%20Angle) (Variables|Default|GetMax%20Fall%20Angle)))
        ;[1 1 1] Close the lid
        (bind _output_get_2 (Variables|Default|SetCurrent%20Angle (+ (Variables|Default|GetCurrent%20Angle) (* (Variables|Default|GetClosing%20Speed) (Variables|Default|GetDelta%20Time))) :!label _label))
        (Transformation|SetRelativeRotation (Variables|Default|GetStaticMesh) (Math|Rotator|MakeRotator _output_get_2 0.0 0.0) false false)
        (else
          ;[1 1 1] Are we trying to close it
          (if (Variables|Default|GetIs%20Closing)
            (if (>= (Variables|Default|GetCurrent%20Angle) (Variables|Default|GetMax%20Fall%20Angle))
              (goto _label))))))
    (else
      ;[1 1 1] Are less than the max angle
      (if (< (Variables|Default|GetCurrent%20Angle) (Variables|Default|GetOpened%20Angle))
        ;[1 1 1] Open the lid
        (bind _output_get_3 (Variables|Default|SetCurrent%20Angle (+ (Variables|Default|GetCurrent%20Angle) (* (Variables|Default|GetOpening%20Speed) (Variables|Default|GetDelta%20Time)))))
        (Transformation|SetRelativeRotation (Variables|Default|GetStaticMesh) (Math|Rotator|MakeRotator _output_get_3 0.0 0.0) false false)))))

(fn ConstructionScript)