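; Air pocket actor with a two-sided water surface, a player blocker and a transition area, whose water level can be moved at runtime.
; The construction script creates dynamic ocean material instances for surface and sub-surface meshes, scales them and applies wave, color and depth settings, negating shore depth below.
; RaiseWater disables blocker and transition collision, moves the root vertically on a timeline while updating the above-water material's height, then restores collision.
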(event Custom|Raise%20Water
  (params (Hight%20to%20change :type Float%20%28single-precision%29))
  (Variables|Default|SetWater%20Displacement Hight%20to%20change)
  (Variables|Default|SetWater%20Last%20Height (Transformation|GetWorldLocation (Variables|Default|GetRoot)))
  ;[1 1 1] Stop the air from pushing
  (Collision|SetCollisionEnabled (Variables|Default|GetPlayer%20Blocker) "NoCollision")
  ;[1 1 1] Move the Air Pocket
  (bind _water_height (Timeline|Water%20Raising PlayFromStart)
    (:Update
      (Transformation|SetWorldLocation (Variables|Default|GetRoot) (+ (Math|Vector|MakeVector 0.0 0.0 (* (Variables|Default|GetWater%20Displacement) _water_height)) (Variables|Default|GetWater%20Last%20Height)) false false)
      ;[1 1 1] Make water visible
      (Rendering|Material|SetScalarParameterValue (Variables|Default|GetAbove%20Water%20Material) "Water Height" (.Z (Math|Vector|BreakVector (Transformation|GetWorldLocation (Variables|Default|GetWaterSurface)))) :!class /Script/Engine.MaterialInstanceDynamic))
    (:Finished
      ;[1 1 1] Store new location
      (Variables|Default|SetWater%20Last%20Height (Transformation|GetWorldLocation (Variables|Default|GetRoot)))
      ;[1 1 1] Resume blocking
      (Collision|SetCollisionEnabled (Variables|Default|GetPlayer%20Blocker) "QueryAndPhysics"))))

(fn ConstructionScript
  (bind _below_water_material (Variables|Default|GetBelow%20Water%20Material))
  (bind _below_water_material_2 (Variables|Default|GetBelow%20Water%20Material))
  (bind _above_water_material (Variables|Default|GetAbove%20Water%20Material))
  (bind _above_water_material_2 (Variables|Default|GetAbove%20Water%20Material))
  (|InitialWaterCreation)
  (for _index (range 0 1)
    (switch int _index
      (:0
        (Rendering|Material|SetScalarParameterValue _above_water_material "Shore Depth" (Variables|Default|GetShore%20Depth) :!class /Script/Engine.MaterialInstanceDynamic)
        (Rendering|Material|SetScalarParameterValue _above_water_material "Wave Speed" (Variables|Default|GetWave%20Speed) :!class /Script/Engine.MaterialInstanceDynamic)
        (Rendering|Material|SetScalarParameterValue _above_water_material "BaseOpacity" (Variables|Default|GetBase%20Opacity) :!class /Script/Engine.MaterialInstanceDynamic)
        (Rendering|Material|SetScalarParameterValue _above_water_material "Water Height" (.Z (Math|Vector|BreakVector (Transformation|GetWorldLocation (Variables|Default|GetWaterSurface)))) :!class /Script/Engine.MaterialInstanceDynamic)
        (Rendering|Material|SetScalarParameterValue _above_water_material "Water Scale" (Variables|Default|GetOverall%20Water%20Scale) :!class /Script/Engine.MaterialInstanceDynamic)
        (Rendering|Material|SetScalarParameterValue _above_water_material "Variation Amount" (Variables|Default|GetVariation%20Amount) :!class /Script/Engine.MaterialInstanceDynamic)
        (Rendering|Material|SetVectorParameterValue _above_water_material "WaterColor A" (Variables|Default|GetPrimary%20Water%20Color) :!class /Script/Engine.MaterialInstanceDynamic)
        (Rendering|Material|SetVectorParameterValue _above_water_material "WaterColor B" (Variables|Default|GetSecondary%20Water%20Color) :!class /Script/Engine.MaterialInstanceDynamic)
        (Rendering|Material|SetScalarParameterValue _above_water_material_2 "Water Depth" (Variables|Default|GetDepth%20Scale) :!class /Script/Engine.MaterialInstanceDynamic)
        (Rendering|Material|SetVectorParameterValue _above_water_material_2 "DeepWater" (Variables|Default|GetDeep%20Water%20Color) :!class /Script/Engine.MaterialInstanceDynamic)
        (Rendering|Material|SetVectorParameterValue _above_water_material_2 "ShallowWater" (Variables|Default|GetShallow%20Water%20Color) :!class /Script/Engine.MaterialInstanceDynamic))
      (:1
        (Rendering|Material|SetScalarParameterValue _below_water_material_2 "Shore Depth" (* (Variables|Default|GetShore%20Depth) -1.0) :!class /Script/Engine.MaterialInstanceDynamic)
        (Rendering|Material|SetScalarParameterValue _below_water_material_2 "Wave Speed" (Variables|Default|GetWave%20Speed) :!class /Script/Engine.MaterialInstanceDynamic)
        (Rendering|Material|SetScalarParameterValue _below_water_material_2 "BaseOpacity" (Variables|Default|GetBase%20Opacity) :!class /Script/Engine.MaterialInstanceDynamic)
        (Rendering|Material|SetScalarParameterValue _below_water_material_2 "Water Height" (.Z (Math|Vector|BreakVector (Transformation|GetWorldLocation (Variables|Default|GetWaterSubSurface)))) :!class /Script/Engine.MaterialInstanceDynamic)
        (Rendering|Material|SetScalarParameterValue _below_water_material_2 "Water Scale" (Variables|Default|GetOverall%20Water%20Scale) :!class /Script/Engine.MaterialInstanceDynamic)
        (Rendering|Material|SetScalarParameterValue _below_water_material_2 "Variation Amount" (Variables|Default|GetVariation%20Amount) :!class /Script/Engine.MaterialInstanceDynamic)
        (Rendering|Material|SetVectorParameterValue _below_water_material_2 "WaterColor A" (Variables|Default|GetPrimary%20Water%20Color) :!class /Script/Engine.MaterialInstanceDynamic)
        (Rendering|Material|SetVectorParameterValue _below_water_material_2 "WaterColor B" (Variables|Default|GetSecondary%20Water%20Color) :!class /Script/Engine.MaterialInstanceDynamic)
        (Rendering|Material|SetScalarParameterValue _below_water_material "Water Depth" (Variables|Default|GetDepth%20Scale) :!class /Script/Engine.MaterialInstanceDynamic)
        (Rendering|Material|SetVectorParameterValue _below_water_material "DeepWater" (Variables|Default|GetDeep%20Water%20Color) :!class /Script/Engine.MaterialInstanceDynamic)
        (Rendering|Material|SetVectorParameterValue _below_water_material "ShallowWater" (Variables|Default|GetShallow%20Water%20Color) :!class /Script/Engine.MaterialInstanceDynamic)))))