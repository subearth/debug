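; VR tablet pickup that shows a four-digit timed security key requested from the moonpool room's control panel.
; Overlapping the screen collider switches that hand to a pointing pose, and leaving reopens it.
; A fingertip on the generate button fetches the key and shows it by swapping number materials on four digit meshes.
; Timers enforce a short cooldown between presses and blank the screen after a few seconds.
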(event OnComponentBeginOverlap(TabletScreenCollider)
  (params (OverlappedComponent :type Primitive%20Component%20Object%20Reference) (OtherActor :type Actor%20Object%20Reference) (OtherComp :type Primitive%20Component%20Object%20Reference) (OtherBodyIndex :type Integer) (bFromSweep :type Boolean) (SweepResult :type Hit%20Result%20Structure%20%28by%20ref%29))
  ;[1 1 1] Control Player hand
  (Player|TrytoPointPlayerFinger OtherComp))

(event OnComponentEndOverlap(GenerateButtonCollider)
  (params (OverlappedComponent :type Primitive%20Component%20Object%20Reference) (OtherActor :type Actor%20Object%20Reference) (OtherComp :type Primitive%20Component%20Object%20Reference) (OtherBodyIndex :type Integer))
  (bind _isplayerfinger (Player|IsPlayerFinger OtherComp))
  (if _isplayerfinger
    _))

(event OnComponentEndOverlap(TabletScreenCollider)
  (params (OverlappedComponent :type Primitive%20Component%20Object%20Reference) (OtherActor :type Actor%20Object%20Reference) (OtherComp :type Primitive%20Component%20Object%20Reference) (OtherBodyIndex :type Integer))
  ;[1 1 1] Control Player hand
  (Player|TrytoOpenPlayerHand OtherComp))

(event OnComponentBeginOverlap(GenerateButtonCollider)
  (params (OverlappedComponent :type Primitive%20Component%20Object%20Reference) (OtherActor :type Actor%20Object%20Reference) (OtherComp :type Primitive%20Component%20Object%20Reference) (OtherBodyIndex :type Integer) (bFromSweep :type Boolean) (SweepResult :type Hit%20Result%20Structure%20%28by%20ref%29))
  (bind _isplayerfinger (Player|IsPlayerFinger OtherComp))
  (if _isplayerfinger
    (Display|TrytoGenerateSecurityKey)))

(event EventBeginPlay
  ;[1 1 1] Get Reference to player character
  (bind _assub_earth_character_new (Utilities|Casting|CastToSubEarthCharacterNew (Game|GetPlayerCharacter 0)))
  (Variables|ExternalReference|SetSubEarthCharacter _assub_earth_character_new)
  (Timer|ClearScreen)
  (bind _asmoonpool_panel (Utilities|Casting|CastToMoonpoolPanel (Variables|/Script/Engine.ChildActorComponent|GetChildActor (Variables|/Game/3D_Assets/Objects/MoonpoolRoom/MoonPoolRoomBP.MoonPoolRoomBP_C|GetControlPanel (Variables|ExternalReference|GetMoonpoolRoomReference)))))
  (Variables|ExternalReference|SetMoonpoolControlPanelReference _asmoonpool_panel))

(event Collision|EventActorBeginOverlap
  (params (OtherActor :type Actor%20Object%20Reference)))

(event EventTick
  (params (DeltaSeconds :type Float%20%28single-precision%29)))

(fn ConstructionScript
  (|CallParentFunction))

(fn DisplayDigitsBaseonString
  (params (SecurityKey :type String))
  ;[1 1 1] Set the display of each digit based on the input string
  (bind _output_get (LocalVariables|Set_SecurityKey SecurityKey))
  (if (== (Utilities|String|Len _output_get) 4)
    (for (_array_element _array_index) (Utilities|String|GetCharacterArrayfromString _output_get)
      (Display|SetDisplayDigittoInt _array_index (Math|Conversions|ToInteger(Byte) _array_element)))))

(fn SetDisplayDigittoInt
  (params (Index :type Integer) (NumToDisplay :type Integer))
  ;[1 1 1] Set individual digit to the correct material
  (for _index (range 0 1)
    (switch int _index
      (:0
        (switch int Index
          (:0
            (LocalVariables|SetMeshToSet (Variables|Default|GetDigit0)))
          (:1
            (LocalVariables|SetMeshToSet (Variables|Default|GetDigit1)))
          (:2
            (LocalVariables|SetMeshToSet (Variables|Default|GetDigit2)))
          (:3
            (LocalVariables|SetMeshToSet (Variables|Default|GetDigit3)))))
      (:1
        (Rendering|Material|SetMaterial (LocalVariables|GetMeshToSet) 0 (Utilities|Array|Get(acopy) (Variables|ExternalReference|GetNumberMaterialReference) NumToDisplay))))))

(fn TrytoOpenPlayerHand
  (params (OtherComp :type Actor%20Component%20Object%20Reference))
  (bind _subearthcharacter (Variables|ExternalReference|GetSubEarthCharacter))
  (if (Components|ComponentHasTag OtherComp "Left Hand Area Collider")
    (Variables|/Game/Blueprints/CharacterBP/SubEarthCharacterNew.SubEarthCharacterNew_C|SetLeft%20Hand%20State _subearthcharacter (Variables|/Game/Blueprints/CharacterBP/SubEarthCharacterNew.SubEarthCharacterNew_C|GetHand%20Open _subearthcharacter))
    (elif (Components|ComponentHasTag OtherComp "Right Hand Area Collider")
      (Variables|/Game/Blueprints/CharacterBP/SubEarthCharacterNew.SubEarthCharacterNew_C|SetRight%20Hand%20State _subearthcharacter (Variables|/Game/Blueprints/CharacterBP/SubEarthCharacterNew.SubEarthCharacterNew_C|GetHand%20Open _subearthcharacter)))))

(fn TrytoPointPlayerFinger
  (params (NewParam :type Actor%20Component%20Object%20Reference))
  (bind _subearthcharacter (Variables|ExternalReference|GetSubEarthCharacter))
  (if (Components|ComponentHasTag NewParam "Left Hand Area Collider")
    (Variables|/Game/Blueprints/CharacterBP/SubEarthCharacterNew.SubEarthCharacterNew_C|SetLeft%20Hand%20State _subearthcharacter (Variables|/Game/Blueprints/CharacterBP/SubEarthCharacterNew.SubEarthCharacterNew_C|GetHand%20Pointing _subearthcharacter))
    (elif (Components|ComponentHasTag NewParam "Right Hand Area Collider")
      (Variables|/Game/Blueprints/CharacterBP/SubEarthCharacterNew.SubEarthCharacterNew_C|SetRight%20Hand%20State _subearthcharacter (Variables|/Game/Blueprints/CharacterBP/SubEarthCharacterNew.SubEarthCharacterNew_C|GetHand%20Pointing _subearthcharacter)))))

(fn IsPlayerFinger
  (params (OtherComp :type Actor%20Component%20Object%20Reference))
  (return (or (Components|ComponentHasTag OtherComp "L_Pointer") (Components|ComponentHasTag OtherComp "R_Pointer"))))

(fn TrytoGenerateSecurityKey
  (if (not (Variables|Default|GetbGeneratorCooldown))
    (bind _key (Default|GenerateTimedSecurityKey (Variables|ExternalReference|GetMoonpoolControlPanelReference)))
    (Display|DisplayDigitsBaseonString _key)
    (Variables|Default|SetbGeneratorCooldown true)
    (Rendering|SetVisibility (Variables|Default|GetDigit0) true false)
    (Utilities|Time|SetTimerbyFunctionName self "GeneratorCooldownEnd" 1.0)
    (Utilities|Time|SetTimerbyFunctionName 0 "ClearScreen" 5.0)))

(fn GeneratorCooldownEnd
  (Variables|Default|SetbGeneratorCooldown false))

(fn ClearScreen
  (Rendering|SetVisibility (Variables|Default|GetDigit0) false false))