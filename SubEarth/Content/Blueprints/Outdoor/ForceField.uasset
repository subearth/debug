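; Outdoor force field actor: a spherical shell of generator pieces around a scaled sphere mesh, with animated spinning rims.
; The construction script spaces generators using a golden-angle Fibonacci sphere with a random index shift, pointing each one's Y axis at the center.
; Those transforms feed instanced rim, center and glass components, and the sphere scales with the field radius.
; Tick rewrites each rim instance's transform to advance its yaw at a constant rate.
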(event EventBeginPlay)

(event Collision|EventActorBeginOverlap
  (params (OtherActor :type Actor%20Object%20Reference)))

(event EventTick
  (params (DeltaSeconds :type Float%20%28single-precision%29))
  (bind _rotatorrim (Variables|Default|GetRotatorRim))
  (Variables|Default|SetDeltaSec DeltaSeconds)
  (for _index (range 0 (Components|InstancedStaticMesh|GetInstanceCount _rotatorrim))
    (Components|InstancedStaticMesh|UpdateInstanceTransform _rotatorrim _index (Math|Transform|MakeTransform (.Location (Math|Transform|BreakTransform (.OutInstanceTransform (Components|InstancedStaticMesh|GetInstanceTransform _rotatorrim _index false)))) (Math|Rotator|MakeRotator (.Roll (Math|Rotator|BreakRotator (.Rotation (Math|Transform|BreakTransform (.OutInstanceTransform (Components|InstancedStaticMesh|GetInstanceTransform _rotatorrim _index false)))))) (.Pitch (Math|Rotator|BreakRotator (.Rotation (Math|Transform|BreakTransform (.OutInstanceTransform (Components|InstancedStaticMesh|GetInstanceTransform _rotatorrim _index false)))))) (+ (.Yaw (Math|Rotator|BreakRotator (.Rotation (Math|Transform|BreakTransform (.OutInstanceTransform (Components|InstancedStaticMesh|GetInstanceTransform _rotatorrim _index false)))))) (* (Variables|Default|GetDeltaSec) 1e+02))) (.Scale (Math|Transform|BreakTransform (.OutInstanceTransform (Components|InstancedStaticMesh|GetInstanceTransform _rotatorrim _index false))))) false false false)))

(fn ConstructionScript
  (bind _forcefieldinstances (Variables|Default|GetForceFieldInstances))
  (LocalVariables|SetForceFieldOffset (/ 2.0 (Math|Conversions|ToFloat(Integer) _forcefieldinstances)))
  (LocalVariables|SetIncrement (Math|Float|MultiplybyPi (- 3.0 (Math|Float|Sqrt 5.0))))
  (LocalVariables|SetRandomNum (* (Math|Random|RandomFloat) (Math|Conversions|ToFloat(Integer) (Variables|Default|GetForceFieldInstances))))
  (for _index (range 0 (- _forcefieldinstances 1))
    (bind _output_get (Variables|Default|Sety (+ (- (* _index (LocalVariables|GetForceFieldOffset)) 1.0) (* (LocalVariables|GetForceFieldOffset) 0.5) 0.0)))
    (LocalVariables|SetR (Math|Float|Sqrt (- 1.0 (* _output_get _output_get))))
    (bind _output_get_2 (LocalVariables|SetPHI (* (Math|Integer|%(Integer) (+ _index (Math|Float|Truncate (LocalVariables|GetRandomNum))) (Variables|Default|GetForceFieldInstances)) (LocalVariables|GetIncrement))))
    (LocalVariables|SetX (* 1.0 (Math|Trig|Cos(Radians) _output_get_2) (LocalVariables|GetR)))
    (LocalVariables|SetZ (* 1.0 (Math|Trig|Sin(Radians) _output_get_2) (LocalVariables|GetR)))
    (Utilities|Array|Add (LocalVariables|GetTransforms) (Math|Transform|MakeTransform (* (Math|Vector|MakeVector (LocalVariables|GetX) (Variables|Default|Gety) (LocalVariables|GetZ)) (Variables|Default|GetForceFieldRadius)) (Math|Rotator|MakeRotfromY (* (Math|Vector|MakeVector (LocalVariables|GetX) (Variables|Default|Gety) (LocalVariables|GetZ)) -1.0)) (Math|Conversions|ToVector(Float) (Variables|Default|GetGeneratorSize)))))
  (for _array_element (LocalVariables|GetTransforms)
    (Components|InstancedStaticMesh|AddInstance (Variables|Default|GetRotatorRim) _array_element)
    (Components|InstancedStaticMesh|AddInstance (Variables|Default|GetRotatorCenter) _array_element)
    (Components|InstancedStaticMesh|AddInstance (Variables|Default|GetGlass) _array_element))
  (Transformation|SetRelativeScale3D (Variables|Default|GetSphere) (Math|Conversions|ToVector(Float) (* (Variables|Default|GetForceFieldRadius) 0.02))))