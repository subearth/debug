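; Outdoor effect set that switches a scene between outdoor and indoor looks, starting in the indoor state.
; Activate and Deactivate toggle atmospheric fog, the caustic light, directional and sky lights, and adjust the referenced post-process bloom and multilayer fog material weight, which is on indoors.
; Tick animates water caustics on a dynamic light-function material by cross-fading consecutive frames of a 64-texture sequence, and prints the blend ratio.
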(event Custom|Event%20Activate
  (bind _indoorpostprocessref (Variables|Default|GetInDoorPostProcessRef))
  (bind _directionallight (Variables|Default|GetDirectionalLight))
  (bind _skylight (Variables|Default|GetSkyLight))
  (bind _lightcomponent (Variables|/Script/Engine.Light|GetLightComponent _directionallight))
  (bind _lightcomponent_2 (Variables|/Script/Engine.SkyLight|GetLightComponent _skylight))
  (bind _postprocess (Variables|/Game/Effects/Lighting/InDoorPostProcess.InDoorPostProcess_C|GetPostProcess _indoorpostprocessref))
  ;[1 1 1] Activate Ourdoor Effects
  (Development|SetHiddeninGame (Variables|Default|GetAtmosphericFog) false false)
  (Variables|Default|SetbIsOutdoor true)
  (Utilities|FlowControl|Sequence
    (:then_0
      ;;[0.1502 0.8398 1] Postprocess
      (if (!= _indoorpostprocessref 0)
        (Development|SetHiddeninGame _postprocess false false)
        (Variables|/Script/Engine.PostProcessComponent|SetSettings _postprocess (Utilities|Struct|MakePostProcessSettings (Variables|Default|GetOutdoorBloomIntensity) (.AmbientCubemapTint (Utilities|Struct|BreakPostProcessSettings (Variables|/Script/Engine.PostProcessComponent|GetSettings _postprocess))) (.AmbientCubemapIntensity (Utilities|Struct|BreakPostProcessSettings (Variables|/Script/Engine.PostProcessComponent|GetSettings _postprocess))) (.AmbientCubemap (Utilities|Struct|BreakPostProcessSettings (Variables|/Script/Engine.PostProcessComponent|GetSettings _postprocess))) (.WeightedBlendables (Utilities|Struct|BreakPostProcessSettings (Variables|/Script/Engine.PostProcessComponent|GetSettings _postprocess)))))
        (Variables|/Script/Engine.PostProcessComponent|SetbEnabled _postprocess true)
        (Utilities|Struct|SetmembersinWeightedBlendable (Utilities|Array|Get(acopy) (Utilities|Struct|BreakWeightedBlendables (Utilities|Struct|BreakPostProcessSettings (Variables|/Script/Engine.PostProcessComponent|GetSettings (Variables|/Game/Effects/Lighting/InDoorPostProcess.InDoorPostProcess_C|GetPostProcess (Variables|Default|GetInDoorPostProcessRef)))))) 0.0 "/Game/Effects/Fog/MultiLayerFogPostProcessMaterial.MultiLayerFogPostProcessMaterial")))
    (:then_2
      (if (!= _directionallight 0)
        (Rendering|SetVisibility _lightcomponent true false)
        (Development|SetHiddeninGame _lightcomponent false false)))
    (:then_3
      (if (!= _skylight 0)
        (Rendering|SetVisibility _lightcomponent_2 true false)
        (Development|SetHiddeninGame _lightcomponent_2 false false)))))

(event Custom|Event%20Deactivate
  (bind _directionallight (Variables|Default|GetDirectionalLight))
  (bind _skylight (Variables|Default|GetSkyLight))
  (bind _indoorpostprocessref (Variables|Default|GetInDoorPostProcessRef))
  (bind _lightcomponent (Variables|/Script/Engine.Light|GetLightComponent _directionallight))
  (bind _lightcomponent_2 (Variables|/Script/Engine.SkyLight|GetLightComponent _skylight))
  (bind _postprocess (Variables|/Game/Effects/Lighting/InDoorPostProcess.InDoorPostProcess_C|GetPostProcess _indoorpostprocessref))
  ;[1 1 1] Deactivate Ourdoor Effects
  (Development|SetHiddeninGame (Variables|Default|GetAtmosphericFog) true true)
  (Variables|Default|SetbIsOutdoor false)
  (Utilities|FlowControl|Sequence
    (:then_0
      ;;[0.1502 0.8398 1] Postprocess
      (if (!= _indoorpostprocessref 0)
        (Development|SetHiddeninGame _postprocess false false)
        (Variables|/Script/Engine.PostProcessComponent|SetSettings _postprocess (Utilities|Struct|MakePostProcessSettings (Variables|Default|GetIndoorBloomIntensity) (.AmbientCubemapTint (Utilities|Struct|BreakPostProcessSettings (Variables|/Script/Engine.PostProcessComponent|GetSettings _postprocess))) (.AmbientCubemapIntensity (Utilities|Struct|BreakPostProcessSettings (Variables|/Script/Engine.PostProcessComponent|GetSettings _postprocess))) (.AmbientCubemap (Utilities|Struct|BreakPostProcessSettings (Variables|/Script/Engine.PostProcessComponent|GetSettings _postprocess))) (.WeightedBlendables (Utilities|Struct|BreakPostProcessSettings (Variables|/Script/Engine.PostProcessComponent|GetSettings _postprocess)))))
        (Variables|/Script/Engine.PostProcessComponent|SetbEnabled _postprocess true)
        (Utilities|Struct|SetmembersinWeightedBlendable (Utilities|Array|Get(acopy) (Utilities|Struct|BreakWeightedBlendables (Utilities|Struct|BreakPostProcessSettings (Variables|/Script/Engine.PostProcessComponent|GetSettings (Variables|/Game/Effects/Lighting/InDoorPostProcess.InDoorPostProcess_C|GetPostProcess (Variables|Default|GetInDoorPostProcessRef)))))) 1.0 "/Game/Effects/Fog/MultiLayerFogPostProcessMaterial.MultiLayerFogPostProcessMaterial")))
    (:then_2
      ;;[1 1 1] HideLights
      (if (!= _directionallight 0)
        (Rendering|SetVisibility _lightcomponent false true)
        (Development|SetHiddeninGame _lightcomponent true false)))
    (:then_3
      (if (!= _skylight 0)
        (Rendering|SetVisibility _lightcomponent_2 false true)
        (Development|SetHiddeninGame _lightcomponent_2 true false)))))

(event EventBeginPlay
  ;[1 1 1] Initial Setup of dynamics materials
  (CallFunction|EventDeactivate)
  (bind _returnvalue (Rendering|Material|CreateDynamicMaterialInstance "/Game/Materials/Caustics/WaterCausticsAnimated.WaterCausticsAnimated" :!class /Script/Engine.KismetMaterialLibrary))
  (bind _output_get (Variables|Default|SetDynamicCausticsVariable _returnvalue))
  (Rendering|Components|Light|SetLightFunctionMaterial (Variables|Default|GetCausticLight) _output_get)
  (Utilities|Struct|SetmembersinWeightedBlendable (Utilities|Array|Get(acopy) (Utilities|Struct|BreakWeightedBlendables (Utilities|Struct|BreakPostProcessSettings (Variables|/Script/Engine.PostProcessComponent|GetSettings (Variables|/Game/Effects/Lighting/InDoorPostProcess.InDoorPostProcess_C|GetPostProcess (Variables|Default|GetInDoorPostProcessRef)))))) 1.0 "/Game/Effects/Fog/MultiLayerFogPostProcessMaterial.MultiLayerFogPostProcessMaterial"))

(event Collision|EventActorBeginOverlap
  (params (OtherActor :type Actor%20Object%20Reference)))

(event EventTick
  (params (DeltaSeconds :type Float%20%28single-precision%29))
  (bind _returnvalue (Utilities|Time|GetGameTimeinSeconds))
  (bind _frequency (Variables|Default|GetFrequency))
  (bind _dynamiccausticsvariable (Variables|Default|GetDynamicCausticsVariable))
  (bind _returnvalue_2 (* _returnvalue _frequency 64.0))
  (bind _remainder (Math|Float|Division(WholeandRemainder) _returnvalue_2 64.0))
  (bind _returnvalue_3 (Math|Float|Truncate _remainder))
  (bind _returnvalue_4 (Math|Float|Fraction _remainder))
  ;[1 1 1] Update Textures of ourdoor caustics
  (if (not (Variables|/Script/Engine.SceneComponent|GetbHiddenInGame (Variables|Default|GetCausticLight)))
    _
    (else
      _))
  (Rendering|Material|SetTextureParameterValue _dynamiccausticsvariable "CausticsTexture" (Utilities|Array|Get(acopy) (Variables|Default|GetTextures) _returnvalue_3))
  (Rendering|Material|SetTextureParameterValue _dynamiccausticsvariable "CausticsTexture_1" (Utilities|Array|Get(acopy) (Variables|Default|GetTextures) (Math|Integer|%(Integer) (+ _returnvalue_3 1) 64)))
  (Rendering|Material|SetScalarParameterValue _dynamiccausticsvariable "TextureLerpRatio" _returnvalue_4 :!class /Script/Engine.MaterialInstanceDynamic)
  (Development|PrintText (Utilities|Text|ToText(Float) _returnvalue_4 "HalfToEven") true true "(R=0.000000,G=0.660000,B=1.000000,A=1.000000)" 0.0))

(fn ConstructionScript)