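; Floatable actor Blueprint that moves its physics mesh vertically, alternating between sinking and floating states.
; BeginPlay gives an initial velocity-change impulse along Z from the current state's speed, then Tick keeps applying that impulse scaled by delta time.
; When vertical velocity nearly reaches zero, Tick flips the state, provided FloatSpeed is positive to start floating or SinkSpeed is negative to start sinking.
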(event EventBeginPlay
  (switch Utilities|FlowControl|Switch|SwitchonFloatingStates (Variables|Default|GetFloat%20State)
    (:NewEnumerator0
      (Physics|AddImpulse (Variables|Default|GetFloating%20Mesh) (Math|Vector|MakeVector 0.0 0.0 (* 1.0 (Variables|Default|GetSink%20Speed))) "None" true))
    (:NewEnumerator1
      (Physics|AddImpulse (Variables|Default|GetFloating%20Mesh) (Math|Vector|MakeVector 0.0 0.0 (* 1.0 (Variables|Default|GetFloat%20Speed))) "None" true))))

(event Collision|EventActorBeginOverlap
  (params (OtherActor :type Actor%20Object%20Reference)))

(event EventTick
  (params (DeltaSeconds :type Float%20%28single-precision%29))
  (Variables|Default|SetTick%20Time DeltaSeconds)
  (switch Utilities|FlowControl|Switch|SwitchonFloatingStates (Variables|Default|GetFloat%20State)
    (:NewEnumerator0
      (Physics|AddImpulse (Variables|Default|GetFloating%20Mesh) (Math|Vector|MakeVector 0.0 0.0 (* (Variables|Default|GetTick%20Time) (Variables|Default|GetSink%20Speed))) "None" true)
      (if (and (< (Math|Float|Absolute(Float) (.Z (Math|Vector|BreakVector (Transformation|GetComponentVelocity (Variables|Default|GetFloating%20Mesh))))) 0.05) (> (Variables|Default|GetFloat%20Speed) 0.0))
        (Variables|Default|SetFloat%20State "NewEnumerator1")))
    (:NewEnumerator1
      (Physics|AddImpulse (Variables|Default|GetFloating%20Mesh) (Math|Vector|MakeVector 0.0 0.0 (* (Variables|Default|GetTick%20Time) (Variables|Default|GetFloat%20Speed))) "None" true)
      (if (and (< (Math|Float|Absolute(Float) (.Z (Math|Vector|BreakVector (Transformation|GetComponentVelocity (Variables|Default|GetFloating%20Mesh))))) 0.05) (< (Variables|Default|GetSink%20Speed) 0.0))
        (Variables|Default|SetFloat%20State "NewEnumerator0")))))

(fn ConstructionScript)