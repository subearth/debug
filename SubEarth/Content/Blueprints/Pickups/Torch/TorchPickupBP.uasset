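; Torch pickup with a point light that can be switched on and off and cycled through colors.
; The down button event flips IsOn and sets the light's visibility to match.
; Right and left button events step LightColorIndex with wraparound, then share one switch that applies green, red, blue or warm white.
; BeginPlay, Tick and construction only call the parent class.
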(event EventBeginPlay
  (|CallParentFunction))

(event Collision|EventActorBeginOverlap
  (params (OtherActor :type Actor%20Object%20Reference)))

(event EventPressButtonDown
  (bind _pointlight (Variables|Default|GetPointLight))
  (if (Variables|Default|GetIs%20On)
    (Variables|Default|SetIs%20On false)
    (Rendering|SetVisibility _pointlight false true)
    (else
      (Variables|Default|SetIs%20On true)
      (Rendering|SetVisibility _pointlight true true))))

(event EventTick
  (params (DeltaSeconds :type Float%20%28single-precision%29))
  (|CallParentFunction DeltaSeconds))

(event EventPressButtonRight
  (params (NewParam :type Boolean))
  (bind _pointlight (Variables|Default|GetPointLight))
  ;[1 1 1] Change Color
  (Variables|Default|SetLight%20Color%20Index (+ (Variables|Default|GetLight%20Color%20Index) 1))
  (if (> (Variables|Default|GetLight%20Color%20Index) (Variables|Default|GetWhite%20Index))
    (Variables|Default|SetLight%20Color%20Index (Variables|Default|GetGreen%20Index)))
  (switch int (Variables|Default|GetLight%20Color%20Index)
    (:0
      (Rendering|Components|Light|SetLightColor _pointlight "(R=0.000000,G=1.000000,B=0.000000,A=1.000000)" true))
    (:1
      (Rendering|Components|Light|SetLightColor _pointlight "(R=1.000000,G=0.000000,B=0.000000,A=1.000000)" true))
    (:2
      (Rendering|Components|Light|SetLightColor _pointlight "(R=0.000000,G=0.000000,B=1.000000,A=1.000000)" true))
    (:3
      (Rendering|Components|Light|SetLightColor _pointlight "(R=0.790000,G=0.594425,B=0.410800,A=1.000000)" true))))

(event EventPressButtonLeft
  (params (NewParam :type Boolean))
  (bind _pointlight (Variables|Default|GetPointLight))
  ;[1 1 1] Change Color
  (Variables|Default|SetLight%20Color%20Index (+ (Variables|Default|GetLight%20Color%20Index) -1))
  (if (< (Variables|Default|GetLight%20Color%20Index) 0)
    (Variables|Default|SetLight%20Color%20Index (Variables|Default|GetWhite%20Index)))
  (switch int (Variables|Default|GetLight%20Color%20Index)
    (:0
      (Rendering|Components|Light|SetLightColor _pointlight "(R=0.000000,G=1.000000,B=0.000000,A=1.000000)" true))
    (:1
      (Rendering|Components|Light|SetLightColor _pointlight "(R=1.000000,G=0.000000,B=0.000000,A=1.000000)" true))
    (:2
      (Rendering|Components|Light|SetLightColor _pointlight "(R=0.000000,G=0.000000,B=1.000000,A=1.000000)" true))
    (:3
      (Rendering|Components|Light|SetLightColor _pointlight "(R=0.790000,G=0.594425,B=0.410800,A=1.000000)" true))))

(fn ConstructionScript
  (|CallParentFunction))