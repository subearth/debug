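; Moonpool control panel puzzle: a touch keypad where the player enters a four-digit code to open the moonpool door.
; Hand-area overlaps switch the character's hands to pointing, and fingertip overlaps press and light keys through a panel state machine that allows one key at a time.
; Enter accepts a default key or a time-stepped code derived from two random constants, then opens the door or briefly shows access denied and resets.
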(event OnComponentEndOverlap(Key3Collider)
  (params (OverlappedComponent :type Primitive%20Component%20Object%20Reference) (OtherActor :type Actor%20Object%20Reference) (OtherComp :type Primitive%20Component%20Object%20Reference) (OtherBodyIndex :type Integer))
  ;[0.1834 0.594 1] Event Handling for keypad
  ;;[1 1 1] Key3
  (bind _isplayerfinger (CallFunction|IsPlayerFinger OtherComp))
  (if _isplayerfinger
    (CallFunction|TrytoReleaseKey "NewEnumerator3")))

(event OnComponentBeginOverlap(Key4Collider)
  (params (OverlappedComponent :type Primitive%20Component%20Object%20Reference) (OtherActor :type Actor%20Object%20Reference) (OtherComp :type Primitive%20Component%20Object%20Reference) (OtherBodyIndex :type Integer) (bFromSweep :type Boolean) (SweepResult :type Hit%20Result%20Structure%20%28by%20ref%29))
  ;[0.1834 0.594 1] Event Handling for keypad
  ;;[1 1 1] Key4
  (bind _isplayerfinger (CallFunction|IsPlayerFinger OtherComp))
  (if _isplayerfinger
    (CallFunction|TrytoPressKey "NewEnumerator4")))

(event OnComponentEndOverlap(Key4Collider)
  (params (OverlappedComponent :type Primitive%20Component%20Object%20Reference) (OtherActor :type Actor%20Object%20Reference) (OtherComp :type Primitive%20Component%20Object%20Reference) (OtherBodyIndex :type Integer))
  ;[0.1834 0.594 1] Event Handling for keypad
  ;;[1 1 1] Key4
  (bind _isplayerfinger (CallFunction|IsPlayerFinger OtherComp))
  (if _isplayerfinger
    (CallFunction|TrytoReleaseKey "NewEnumerator4")))

(event OnComponentBeginOverlap(KeyEnterCollider)
  (params (OverlappedComponent :type Primitive%20Component%20Object%20Reference) (OtherActor :type Actor%20Object%20Reference) (OtherComp :type Primitive%20Component%20Object%20Reference) (OtherBodyIndex :type Integer) (bFromSweep :type Boolean) (SweepResult :type Hit%20Result%20Structure%20%28by%20ref%29))
  ;[0.1834 0.594 1] Event Handling for keypad
  ;;[1 1 1] Key Enter
  (bind _isplayerfinger (CallFunction|IsPlayerFinger OtherComp))
  (if _isplayerfinger
    (CallFunction|TrytoPressKey "NewEnumerator11")))

(event OnComponentEndOverlap(KeyEnterCollider)
  (params (OverlappedComponent :type Primitive%20Component%20Object%20Reference) (OtherActor :type Actor%20Object%20Reference) (OtherComp :type Primitive%20Component%20Object%20Reference) (OtherBodyIndex :type Integer))
  ;[0.1834 0.594 1] Event Handling for keypad
  ;;[1 1 1] Key Enter
  (bind _isplayerfinger (CallFunction|IsPlayerFinger OtherComp))
  (if _isplayerfinger
    (CallFunction|TrytoReleaseKey "NewEnumerator11")))

(event OnComponentEndOverlap(KeyPadCollider)
  (params (OverlappedComponent :type Primitive%20Component%20Object%20Reference) (OtherActor :type Actor%20Object%20Reference) (OtherComp :type Primitive%20Component%20Object%20Reference) (OtherBodyIndex :type Integer))
  ;[1 1 1] ControlPlayerHand
  (CallFunction|TrytoOpenPlayerHand OtherComp))

(event OnComponentBeginOverlap(KeyBackspaceCollider)
  (params (OverlappedComponent :type Primitive%20Component%20Object%20Reference) (OtherActor :type Actor%20Object%20Reference) (OtherComp :type Primitive%20Component%20Object%20Reference) (OtherBodyIndex :type Integer) (bFromSweep :type Boolean) (SweepResult :type Hit%20Result%20Structure%20%28by%20ref%29))
  ;[0.1834 0.594 1] Event Handling for keypad
  ;;[1 1 1] Backspace
  (bind _isplayerfinger (CallFunction|IsPlayerFinger OtherComp))
  (if _isplayerfinger
    (CallFunction|TrytoPressKey "NewEnumerator10")))

(event OnComponentEndOverlap(KeyBackspaceCollider)
  (params (OverlappedComponent :type Primitive%20Component%20Object%20Reference) (OtherActor :type Actor%20Object%20Reference) (OtherComp :type Primitive%20Component%20Object%20Reference) (OtherBodyIndex :type Integer))
  ;[0.1834 0.594 1] Event Handling for keypad
  ;;[1 1 1] Backspace
  (bind _isplayerfinger (CallFunction|IsPlayerFinger OtherComp))
  (if _isplayerfinger
    (CallFunction|TrytoReleaseKey "NewEnumerator10")))

(event OnComponentBeginOverlap(Key5Collider)
  (params (OverlappedComponent :type Primitive%20Component%20Object%20Reference) (OtherActor :type Actor%20Object%20Reference) (OtherComp :type Primitive%20Component%20Object%20Reference) (OtherBodyIndex :type Integer) (bFromSweep :type Boolean) (SweepResult :type Hit%20Result%20Structure%20%28by%20ref%29))
  ;[0.1834 0.594 1] Event Handling for keypad
  ;;[1 1 1] Key5
  (bind _isplayerfinger (CallFunction|IsPlayerFinger OtherComp))
  (if _isplayerfinger
    (CallFunction|TrytoPressKey "NewEnumerator5")))

(event OnComponentEndOverlap(Key5Collider)
  (params (OverlappedComponent :type Primitive%20Component%20Object%20Reference) (OtherActor :type Actor%20Object%20Reference) (OtherComp :type Primitive%20Component%20Object%20Reference) (OtherBodyIndex :type Integer))
  ;[0.1834 0.594 1] Event Handling for keypad
  ;;[1 1 1] Key5
  (bind _isplayerfinger (CallFunction|IsPlayerFinger OtherComp))
  (if _isplayerfinger
    (CallFunction|TrytoReleaseKey "NewEnumerator5")))

(event OnComponentBeginOverlap(Key1Collider)
  (params (OverlappedComponent :type Primitive%20Component%20Object%20Reference) (OtherActor :type Actor%20Object%20Reference) (OtherComp :type Primitive%20Component%20Object%20Reference) (OtherBodyIndex :type Integer) (bFromSweep :type Boolean) (SweepResult :type Hit%20Result%20Structure%20%28by%20ref%29))
  ;[0.1834 0.594 1] Event Handling for keypad
  ;;[1 1 1] Key1
  (bind _isplayerfinger (CallFunction|IsPlayerFinger OtherComp))
  (if _isplayerfinger
    (CallFunction|TrytoPressKey "NewEnumerator1")))

(event OnComponentBeginOverlap(Key6Collider)
  (params (OverlappedComponent :type Primitive%20Component%20Object%20Reference) (OtherActor :type Actor%20Object%20Reference) (OtherComp :type Primitive%20Component%20Object%20Reference) (OtherBodyIndex :type Integer) (bFromSweep :type Boolean) (SweepResult :type Hit%20Result%20Structure%20%28by%20ref%29))
  ;[0.1834 0.594 1] Event Handling for keypad
  ;;[1 1 1] Key6
  (bind _isplayerfinger (CallFunction|IsPlayerFinger OtherComp))
  (if _isplayerfinger
    (CallFunction|TrytoPressKey "NewEnumerator6")))

(event OnComponentEndOverlap(Key6Collider)
  (params (OverlappedComponent :type Primitive%20Component%20Object%20Reference) (OtherActor :type Actor%20Object%20Reference) (OtherComp :type Primitive%20Component%20Object%20Reference) (OtherBodyIndex :type Integer))
  ;[0.1834 0.594 1] Event Handling for keypad
  ;;[1 1 1] Key6
  (bind _isplayerfinger (CallFunction|IsPlayerFinger OtherComp))
  (if _isplayerfinger
    (CallFunction|TrytoReleaseKey "NewEnumerator6")))

(event OnComponentBeginOverlap(KeyPadCollider)
  (params (OverlappedComponent :type Primitive%20Component%20Object%20Reference) (OtherActor :type Actor%20Object%20Reference) (OtherComp :type Primitive%20Component%20Object%20Reference) (OtherBodyIndex :type Integer) (bFromSweep :type Boolean) (SweepResult :type Hit%20Result%20Structure%20%28by%20ref%29))
  ;[1 1 1] ControlPlayerHand
  (CallFunction|TrytoPointPlayerFinger OtherComp))

(event OnComponentBeginOverlap(Key7Collider)
  (params (OverlappedComponent :type Primitive%20Component%20Object%20Reference) (OtherActor :type Actor%20Object%20Reference) (OtherComp :type Primitive%20Component%20Object%20Reference) (OtherBodyIndex :type Integer) (bFromSweep :type Boolean) (SweepResult :type Hit%20Result%20Structure%20%28by%20ref%29))
  ;[0.1834 0.594 1] Event Handling for keypad
  ;;[1 1 1] Key7
  (bind _isplayerfinger (CallFunction|IsPlayerFinger OtherComp))
  (if _isplayerfinger
    (CallFunction|TrytoPressKey "NewEnumerator7")))

(event OnComponentEndOverlap(Key7Collider)
  (params (OverlappedComponent :type Primitive%20Component%20Object%20Reference) (OtherActor :type Actor%20Object%20Reference) (OtherComp :type Primitive%20Component%20Object%20Reference) (OtherBodyIndex :type Integer))
  ;[0.1834 0.594 1] Event Handling for keypad
  ;;[1 1 1] Key7
  (bind _isplayerfinger (CallFunction|IsPlayerFinger OtherComp))
  (if _isplayerfinger
    (CallFunction|TrytoReleaseKey "NewEnumerator7")))

(event OnComponentEndOverlap(Key8Collider)
  (params (OverlappedComponent :type Primitive%20Component%20Object%20Reference) (OtherActor :type Actor%20Object%20Reference) (OtherComp :type Primitive%20Component%20Object%20Reference) (OtherBodyIndex :type Integer))
  ;[0.1834 0.594 1] Event Handling for keypad
  ;;[1 1 1] Key8
  (bind _isplayerfinger (CallFunction|IsPlayerFinger OtherComp))
  (if _isplayerfinger
    (CallFunction|TrytoReleaseKey "NewEnumerator8")))

(event OnComponentBeginOverlap(Key8Collider)
  (params (OverlappedComponent :type Primitive%20Component%20Object%20Reference) (OtherActor :type Actor%20Object%20Reference) (OtherComp :type Primitive%20Component%20Object%20Reference) (OtherBodyIndex :type Integer) (bFromSweep :type Boolean) (SweepResult :type Hit%20Result%20Structure%20%28by%20ref%29))
  ;[0.1834 0.594 1] Event Handling for keypad
  ;;[1 1 1] Key8
  (bind _isplayerfinger (CallFunction|IsPlayerFinger OtherComp))
  (if _isplayerfinger
    (CallFunction|TrytoPressKey "NewEnumerator8")))

(event OnComponentEndOverlap(Key1Collider)
  (params (OverlappedComponent :type Primitive%20Component%20Object%20Reference) (OtherActor :type Actor%20Object%20Reference) (OtherComp :type Primitive%20Component%20Object%20Reference) (OtherBodyIndex :type Integer))
  ;[0.1834 0.594 1] Event Handling for keypad
  ;;[1 1 1] Key1
  (bind _isplayerfinger (CallFunction|IsPlayerFinger OtherComp))
  (if _isplayerfinger
    (CallFunction|TrytoReleaseKey "NewEnumerator1")))

(event OnComponentBeginOverlap(Key9Collider)
  (params (OverlappedComponent :type Primitive%20Component%20Object%20Reference) (OtherActor :type Actor%20Object%20Reference) (OtherComp :type Primitive%20Component%20Object%20Reference) (OtherBodyIndex :type Integer) (bFromSweep :type Boolean) (SweepResult :type Hit%20Result%20Structure%20%28by%20ref%29))
  ;[0.1834 0.594 1] Event Handling for keypad
  ;;[1 1 1] Key9
  (bind _isplayerfinger (CallFunction|IsPlayerFinger OtherComp))
  (if _isplayerfinger
    (CallFunction|TrytoPressKey "NewEnumerator9")))

(event OnComponentEndOverlap(Key9Collider)
  (params (OverlappedComponent :type Primitive%20Component%20Object%20Reference) (OtherActor :type Actor%20Object%20Reference) (OtherComp :type Primitive%20Component%20Object%20Reference) (OtherBodyIndex :type Integer))
  ;[0.1834 0.594 1] Event Handling for keypad
  ;;[1 1 1] Key9
  (bind _isplayerfinger (CallFunction|IsPlayerFinger OtherComp))
  (if _isplayerfinger
    (CallFunction|TrytoReleaseKey "NewEnumerator9")))

(event OnComponentBeginOverlap(Key2Collider)
  (params (OverlappedComponent :type Primitive%20Component%20Object%20Reference) (OtherActor :type Actor%20Object%20Reference) (OtherComp :type Primitive%20Component%20Object%20Reference) (OtherBodyIndex :type Integer) (bFromSweep :type Boolean) (SweepResult :type Hit%20Result%20Structure%20%28by%20ref%29))
  ;[0.1834 0.594 1] Event Handling for keypad
  ;;[1 1 1] Key2
  (bind _isplayerfinger (CallFunction|IsPlayerFinger OtherComp))
  (if _isplayerfinger
    (CallFunction|TrytoPressKey "NewEnumerator2")))

(event OnComponentBeginOverlap(Key0Collider)
  (params (OverlappedComponent :type Primitive%20Component%20Object%20Reference) (OtherActor :type Actor%20Object%20Reference) (OtherComp :type Primitive%20Component%20Object%20Reference) (OtherBodyIndex :type Integer) (bFromSweep :type Boolean) (SweepResult :type Hit%20Result%20Structure%20%28by%20ref%29))
  ;[0.1834 0.594 1] Event Handling for keypad
  ;;[1 1 1] Key0
  (bind _isplayerfinger (CallFunction|IsPlayerFinger OtherComp))
  (if _isplayerfinger
    (CallFunction|TrytoPressKey "NewEnumerator0")))

(event OnComponentEndOverlap(Key0Collider)
  (params (OverlappedComponent :type Primitive%20Component%20Object%20Reference) (OtherActor :type Actor%20Object%20Reference) (OtherComp :type Primitive%20Component%20Object%20Reference) (OtherBodyIndex :type Integer))
  ;[0.1834 0.594 1] Event Handling for keypad
  ;;[1 1 1] Key0
  (bind _isplayerfinger (CallFunction|IsPlayerFinger OtherComp))
  (if _isplayerfinger
    (CallFunction|TrytoReleaseKey "NewEnumerator0")))

(event OnComponentEndOverlap(Key2Collider)
  (params (OverlappedComponent :type Primitive%20Component%20Object%20Reference) (OtherActor :type Actor%20Object%20Reference) (OtherComp :type Primitive%20Component%20Object%20Reference) (OtherBodyIndex :type Integer))
  ;[0.1834 0.594 1] Event Handling for keypad
  ;;[1 1 1] Key2
  (bind _isplayerfinger (CallFunction|IsPlayerFinger OtherComp))
  (if _isplayerfinger
    (CallFunction|TrytoReleaseKey "NewEnumerator2")))

(event OnComponentBeginOverlap(Key3Collider)
  (params (OverlappedComponent :type Primitive%20Component%20Object%20Reference) (OtherActor :type Actor%20Object%20Reference) (OtherComp :type Primitive%20Component%20Object%20Reference) (OtherBodyIndex :type Integer) (bFromSweep :type Boolean) (SweepResult :type Hit%20Result%20Structure%20%28by%20ref%29))
  ;[0.1834 0.594 1] Event Handling for keypad
  ;;[1 1 1] Key3
  (bind _isplayerfinger (CallFunction|IsPlayerFinger OtherComp))
  (if _isplayerfinger
    (CallFunction|TrytoPressKey "NewEnumerator3")))

(event EventBeginPlay
  ;[1 1 1] Get Reference to player character
  (bind _assub_earth_character_new (Utilities|Casting|CastToSubEarthCharacterNew (Game|GetPlayerCharacter 0)))
  (Variables|ExternalReference|SetSubEarthCharacter _assub_earth_character_new)
  (Variables|Default|SetControlPanelState "NewEnumerator0")
  (Variables|SecurityKeyGeneration|SetSecureKeyConstA (Math|Random|RandomInteger 4093))
  (Variables|SecurityKeyGeneration|SetSecureKeyConstB (Math|Random|RandomInteger 4093)))

(event Collision|EventActorBeginOverlap
  (params (OtherActor :type Actor%20Object%20Reference)))

(event EventTick
  (params (DeltaSeconds :type Float%20%28single-precision%29)))

(fn ConstructionScript
  (bind _digitnumberarray (Variables|Input|GetDigitNumberArray))
  (bind _digit0 (Variables|Default|GetDigit0))
  (bind _digit1 (Variables|Default|GetDigit1))
  (bind _digit2 (Variables|Default|GetDigit2))
  (bind _digit3 (Variables|Default|GetDigit3))
  (for _index (range 0 4)
    (switch int _index
      (:0
        ;[1 1 1] Initialize Digit Number Array
        (Utilities|Array|Clear _digitnumberarray)
        (Rendering|SetVisibility _digit0 false false)
        (Utilities|Array|Add _digitnumberarray _digit0)
        (Rendering|SetVisibility _digit1 false false)
        (Utilities|Array|Add _digitnumberarray _digit1)
        (Rendering|SetVisibility _digit2 false false)
        (Utilities|Array|Add _digitnumberarray _digit2)
        (Rendering|SetVisibility _digit3 false false)
        (Utilities|Array|Add _digitnumberarray _digit3)
        (Variables|Input|SetNextDigitIndex 0)))))

(fn TrytoPointPlayerFinger
  (params (ComponentToTest :type Actor%20Component%20Object%20Reference))
  (bind _subearthcharacter (Variables|ExternalReference|GetSubEarthCharacter))
  (if (Components|ComponentHasTag ComponentToTest "Left Hand Area Collider")
    (Variables|/Game/Blueprints/CharacterBP/SubEarthCharacterNew.SubEarthCharacterNew_C|SetLeft%20Hand%20State _subearthcharacter (Variables|/Game/Blueprints/CharacterBP/SubEarthCharacterNew.SubEarthCharacterNew_C|GetHand%20Pointing _subearthcharacter))
    (elif (Components|ComponentHasTag ComponentToTest "Right Hand Area Collider")
      (Variables|/Game/Blueprints/CharacterBP/SubEarthCharacterNew.SubEarthCharacterNew_C|SetRight%20Hand%20State _subearthcharacter (Variables|/Game/Blueprints/CharacterBP/SubEarthCharacterNew.SubEarthCharacterNew_C|GetHand%20Pointing _subearthcharacter)))))

(fn TrytoOpenPlayerHand
  (params (ComponentToTest :type Actor%20Component%20Object%20Reference))
  (bind _subearthcharacter (Variables|ExternalReference|GetSubEarthCharacter))
  (if (Components|ComponentHasTag ComponentToTest "Left Hand Area Collider")
    (Variables|/Game/Blueprints/CharacterBP/SubEarthCharacterNew.SubEarthCharacterNew_C|SetLeft%20Hand%20State _subearthcharacter (Variables|/Game/Blueprints/CharacterBP/SubEarthCharacterNew.SubEarthCharacterNew_C|GetHand%20Open _subearthcharacter))
    (elif (Components|ComponentHasTag ComponentToTest "Right Hand Area Collider")
      (Variables|/Game/Blueprints/CharacterBP/SubEarthCharacterNew.SubEarthCharacterNew_C|SetRight%20Hand%20State _subearthcharacter (Variables|/Game/Blueprints/CharacterBP/SubEarthCharacterNew.SubEarthCharacterNew_C|GetHand%20Open _subearthcharacter)))))

(fn TrytoPressKey
  (params (Key :type EMoonpoolControlPanelKeys%20Enum))
  (bind _nextdigitindex (Variables|Input|GetNextDigitIndex))
  (bind _digitnumberarray (Variables|Input|GetDigitNumberArray))
  (bind _item (Utilities|Array|Get(acopy) _digitnumberarray _nextdigitindex))
  (if (== (Variables|Default|GetControlPanelState) (Utilities|Enum|LiteralenumEMoonpoolControlPanelState "NewEnumerator0"))
    (Variables|Default|SetControlPanelState "NewEnumerator1")
    (bind _output_get (Variables|Input|SetCurrentPressedKey Key))
    (CallFunction|LightUpKey _output_get)
    (switch Utilities|FlowControl|Switch|SwitchonEMoonpoolControlPanelKeys (Variables|Input|GetCurrentPressedKey)
      (:NewEnumerator0
        ;[1 1 1] Toggle the next number on
        (LocalVariables|SetNumberPressed 0)
        (if (and (>= (Variables|Input|GetNextDigitIndex) 0) (<= (Variables|Input|GetNextDigitIndex) 3)) :!label _label
          (Rendering|Material|SetMaterial _item 0 (Utilities|Array|Get(acopy) (Variables|Input|GetKeyMaterialReferences) (LocalVariables|GetNumberPressed)))
          (Rendering|SetVisibility _item true false)
          (Math|Integer|IncrementInt (Variables|Input|GetNextDigitIndex)
            (:%20%20
              (bind _output_get_2 (Variables|Input|SetCachedInput (Utilities|String|Append (Variables|Input|GetCachedInput) (Utilities|String|ToString(Integer) (LocalVariables|GetNumberPressed)))))))))
      (:NewEnumerator1
        (LocalVariables|SetNumberPressed 1)
        (goto _label))
      (:NewEnumerator2
        (LocalVariables|SetNumberPressed 2)
        (goto _label))
      (:NewEnumerator3
        (LocalVariables|SetNumberPressed 3)
        (goto _label))
      (:NewEnumerator4
        (LocalVariables|SetNumberPressed 4)
        (goto _label))
      (:NewEnumerator5
        (LocalVariables|SetNumberPressed 5)
        (goto _label))
      (:NewEnumerator6
        (LocalVariables|SetNumberPressed 6)
        (goto _label))
      (:NewEnumerator7
        (LocalVariables|SetNumberPressed 7)
        (goto _label))
      (:NewEnumerator8
        (LocalVariables|SetNumberPressed 8)
        (goto _label))
      (:NewEnumerator9
        (LocalVariables|SetNumberPressed 9)
        (goto _label))
      (:NewEnumerator10
        ;[1 1 1] Hide the deleted number
        (if (and (>= (- (Variables|Input|GetNextDigitIndex) 1) 0) (<= (- (Variables|Input|GetNextDigitIndex) 1) 3))
          (Rendering|SetVisibility (Utilities|Array|Get(acopy) (Variables|Input|GetDigitNumberArray) (- (Variables|Input|GetNextDigitIndex) 1)) false false)
          (Math|Integer|DecrementInt (Variables|Input|GetNextDigitIndex)
            (:%20%20
              (bind _output_get_3 (Variables|Input|SetCachedInput (Utilities|String|LeftChop (Variables|Input|GetCachedInput) 1)))))))
      (:NewEnumerator11
        ;[1 1 1] Check the security code
        (if (== (Variables|Input|GetNextDigitIndex) 4)
          (bind _iscorrectsecuritykey (CallFunction|IsCorrectSecurityKey))
          (if _iscorrectsecuritykey
            ;;[1 1 1] If correct, grant access
            (Rendering|Material|SetMaterial (Variables|Default|GetControlPanelScreenMessage) 0 "/Game/Materials/ControlPanelA/MoonpoolAccessGranted_Mat.MoonpoolAccessGranted_Mat")
            (Variables|Default|SetControlPanelState "NewEnumerator3")
            (Rendering|SetVisibility (Variables|Default|GetControlPanelScreenMessage) true false)
            (Rendering|SetVisibility (Variables|Default|GetDisplay) false true)
            (Rendering|SetVisibility (Variables|Default|GetKeyPad) false true)
            (Default|EventOpenMoonpoolDoor (Variables|ExternalReference|GetMoonpoolRoomReference))
            (else
              ;;[1 1 1] If wrong, clear the input cache and reset digits
              (CallFunction|EnterWarningState)
              (CallFunction|TrytoReleaseKey "NewEnumerator11"))))))))

(fn IsCorrectSecurityKey
  (bind _defaultsecuritykey (Variables|Input|GetDefaultSecurityKey))
  (bind _cachedinput (Variables|Input|GetCachedInput))
  (bind _key (CallFunction|GenerateTimedSecurityKey))
  (Development|PrintString (Utilities|String|Append "DEBUG:: Comparing Input:" _cachedinput " with default key " _defaultsecuritykey " or generated key " _key " result is " (Utilities|String|ToString(Boolean) (or (Utilities|Enum|Equal(Enum) _key (Variables|Input|GetCachedInput)) (Utilities|Enum|Equal(Enum) _defaultsecuritykey _cachedinput)))) false true "(R=1.000000,G=0.000000,B=0.077258,A=1.000000)")
  (return (or (Utilities|Enum|Equal(Enum) _key (Variables|Input|GetCachedInput)) (Utilities|Enum|Equal(Enum) _defaultsecuritykey _cachedinput))))

(fn TrytoReleaseKey
  (params (KeyToRelease :type EMoonpoolControlPanelKeys%20Enum))
  (if (Utilities|Enum|Equal(Enum) KeyToRelease (Variables|Input|GetCurrentPressedKey))
    (switch Utilities|FlowControl|Switch|SwitchonEMoonpoolControlPanelState (Variables|Default|GetControlPanelState)
      (:NewEnumerator1
        (Variables|Default|SetControlPanelState "NewEnumerator0"))
      (:NewEnumerator3
        _))
    (CallFunction|LightOffKey (Variables|Input|GetCurrentPressedKey))
    (Variables|Input|SetCurrentPressedKey "NewEnumerator12")))

(fn IsPlayerFinger
  (params (Component :type Actor%20Component%20Object%20Reference))
  (return (or (Components|ComponentHasTag Component "L_Pointer") (Components|ComponentHasTag Component "R_Pointer"))))

(fn GenerateTimedSecurityKey
  (return (Utilities|String|ToString(Integer) (Math|Integer|%(Integer) (* (+ (Variables|SecurityKeyGeneration|GetSecureKeyConstA) (Math|Float|Floor (/ (Utilities|Time|GetGameTimeinSeconds) (Variables|Input|GetSecurityTimeStep)))) (Variables|SecurityKeyGeneration|GetSecureKeyConstB)) 10000))))

(fn ResetInput
  (for _array_element (Variables|Input|GetDigitNumberArray)
    (Rendering|SetVisibility _array_element false false))
  (Variables|Input|SetNextDigitIndex 0)
  (Variables|Input|SetCachedInput ""))

(fn EndWarningState
  (if (Utilities|Enum|Equal(Enum) (Variables|Default|GetControlPanelState) "NewEnumerator5")
    (Rendering|SetVisibility (Variables|Default|GetControlPanelScreenMessage) false false)
    (Rendering|Material|SetMaterial (Variables|Default|GetControlPanelScreen) 0 "/Game/Materials/ControlPanelA/MoonpoolBaseCLR_Mat.MoonpoolBaseCLR_Mat")
    (Variables|Default|SetControlPanelState "NewEnumerator0")
    (Rendering|SetVisibility (Variables|Default|GetDisplay) true false)
    (Rendering|SetVisibility (Variables|Default|GetKeyPad) true true)))

(fn EnterWarningState
  (Rendering|Material|SetMaterial (Variables|Default|GetControlPanelScreenMessage) 0 "/Game/Materials/ControlPanelA/MoonpoolAccessDenied_Mat.MoonpoolAccessDenied_Mat")
  (Rendering|SetVisibility (Variables|Default|GetControlPanelScreenMessage) true false)
  (Rendering|SetVisibility (Variables|Default|GetDisplay) false true)
  (Rendering|SetVisibility (Variables|Default|GetKeyPad) false true)
  (CallFunction|ResetInput)
  (Variables|Default|SetControlPanelState "NewEnumerator5")
  (bind _returnvalue (Utilities|Time|SetTimerbyFunctionName self "EndWarningState" 2.0))
  (Variables|Default|SetWarningTimerHandle _returnvalue))

(fn LightUpKey
  (params (KeyPressed :type EMoonpoolControlPanelKeys%20Enum))
  (switch Utilities|FlowControl|Switch|SwitchonEMoonpoolControlPanelKeys KeyPressed
    (:NewEnumerator0
      (Rendering|Material|SetMaterial (Variables|Default|GetKey0) 0 "/Game/Materials/ControlPanelA/PadNumberKeyPressed_Mat_InstNum0.PadNumberKeyPressed_Mat_InstNum0"))
    (:NewEnumerator1
      (Rendering|Material|SetMaterial (Variables|Default|GetKey1) 0 "/Game/Materials/ControlPanelA/PadNumberKeyPressed_Mat_InstNum1.PadNumberKeyPressed_Mat_InstNum1"))
    (:NewEnumerator2
      (Rendering|Material|SetMaterial (Variables|Default|GetKey2) 0 "/Game/Materials/ControlPanelA/PadNumberKeyPressed_Mat_InstNum2.PadNumberKeyPressed_Mat_InstNum2"))
    (:NewEnumerator3
      (Rendering|Material|SetMaterial (Variables|Default|GetKey3) 0 "/Game/Materials/ControlPanelA/PadNumberKeyPressed_Mat_InstNum3.PadNumberKeyPressed_Mat_InstNum3"))
    (:NewEnumerator4
      (Rendering|Material|SetMaterial (Variables|Default|GetKey4) 0 "/Game/Materials/ControlPanelA/PadNumberKeyPressed_Mat_InstNum4.PadNumberKeyPressed_Mat_InstNum4"))
    (:NewEnumerator5
      (Rendering|Material|SetMaterial (Variables|Default|GetKey5) 0 "/Game/Materials/ControlPanelA/PadNumberKeyPressed_Mat_InstNum5.PadNumberKeyPressed_Mat_InstNum5"))
    (:NewEnumerator6
      (Rendering|Material|SetMaterial (Variables|Default|GetKey6) 0 "/Game/Materials/ControlPanelA/PadNumberKeyPressed_Mat_InstNum6.PadNumberKeyPressed_Mat_InstNum6"))
    (:NewEnumerator7
      (Rendering|Material|SetMaterial (Variables|Default|GetKey7) 0 "/Game/Materials/ControlPanelA/PadNumberKeyPressed_Mat_InstNum7.PadNumberKeyPressed_Mat_InstNum7"))
    (:NewEnumerator8
      (Rendering|Material|SetMaterial (Variables|Default|GetKey8) 0 "/Game/Materials/ControlPanelA/PadNumberKeyPressed_Mat_InstNum8.PadNumberKeyPressed_Mat_InstNum8"))
    (:NewEnumerator9
      (Rendering|Material|SetMaterial (Variables|Default|GetKey9) 0 "/Game/Materials/ControlPanelA/PadNumberKeyPressed_Mat_InstNum9.PadNumberKeyPressed_Mat_InstNum9"))
    (:NewEnumerator10
      (Rendering|Material|SetMaterial (Variables|Default|GetKeyBackspace) 0 "/Game/Materials/ControlPanelA/PadNumberKeyPressed_Mat_InstBackspace.PadNumberKeyPressed_Mat_InstBackspace"))
    (:NewEnumerator11
      (Rendering|Material|SetMaterial (Variables|Default|GetKeyEnter) 0 "/Game/Materials/ControlPanelA/PadNumberKeyPressed_Mat_InstEnter.PadNumberKeyPressed_Mat_InstEnter"))))

(fn LightOffKey
  (params (KeyToDim :type EMoonpoolControlPanelKeys%20Enum))
  (switch Utilities|FlowControl|Switch|SwitchonEMoonpoolControlPanelKeys KeyToDim
    (:NewEnumerator0
      (Rendering|Material|SetMaterial (Variables|Default|GetKey0) 0 "/Game/Materials/ControlPanelA/PadNumberKey_Mat_InstNum0.PadNumberKey_Mat_InstNum0"))
    (:NewEnumerator1
      (Rendering|Material|SetMaterial (Variables|Default|GetKey1) 0 "/Game/Materials/ControlPanelA/PadNumberKey_Mat_InstNum1.PadNumberKey_Mat_InstNum1"))
    (:NewEnumerator2
      (Rendering|Material|SetMaterial (Variables|Default|GetKey2) 0 "/Game/Materials/ControlPanelA/PadNumberKey_Mat_InstNum2.PadNumberKey_Mat_InstNum2"))
    (:NewEnumerator3
      (Rendering|Material|SetMaterial (Variables|Default|GetKey3) 0 "/Game/Materials/ControlPanelA/PadNumberKey_Mat_InstNum3.PadNumberKey_Mat_InstNum3"))
    (:NewEnumerator4
      (Rendering|Material|SetMaterial (Variables|Default|GetKey4) 0 "/Game/Materials/ControlPanelA/PadNumberKey_Mat_InstNum4.PadNumberKey_Mat_InstNum4"))
    (:NewEnumerator5
      (Rendering|Material|SetMaterial (Variables|Default|GetKey5) 0 "/Game/Materials/ControlPanelA/PadNumberKey_Mat_InstNum5.PadNumberKey_Mat_InstNum5"))
    (:NewEnumerator6
      (Rendering|Material|SetMaterial (Variables|Default|GetKey6) 0 "/Game/Materials/ControlPanelA/PadNumberKey_Mat_InstNum6.PadNumberKey_Mat_InstNum6"))
    (:NewEnumerator7
      (Rendering|Material|SetMaterial (Variables|Default|GetKey7) 0 "/Game/Materials/ControlPanelA/PadNumberKey_Mat_InstNum7.PadNumberKey_Mat_InstNum7"))
    (:NewEnumerator8
      (Rendering|Material|SetMaterial (Variables|Default|GetKey8) 0 "/Game/Materials/ControlPanelA/PadNumberKey_Mat_InstNum8.PadNumberKey_Mat_InstNum8"))
    (:NewEnumerator9
      (Rendering|Material|SetMaterial (Variables|Default|GetKey9) 0 "/Game/Materials/ControlPanelA/PadNumberKey_Mat_InstNum9.PadNumberKey_Mat_InstNum9"))
    (:NewEnumerator10
      (Rendering|Material|SetMaterial (Variables|Default|GetKeyBackspace) 0 "/Game/Materials/ControlPanelA/PadKeyBackspace_Mat.PadKeyBackspace_Mat"))
    (:NewEnumerator11
      (Rendering|Material|SetMaterial (Variables|Default|GetKeyEnter) 0 "/Game/Materials/ControlPanelA/PadNumberKey_Mat_InstEnter.PadNumberKey_Mat_InstEnter"))))